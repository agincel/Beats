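; Player pawn for a lane-based rhythm game that turns keyboard input into note-highway presses and song control.
; Four lane input actions call ActivateLane on press and release, which forwards the lane index and pressed state to every Highway actor in the level.
; Space calls Begin on every BeatPuppeteer, and Escape quits the game.
; Targets are looked up with GetAllActorsOfClass on each input rather than cached.
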(event Input|ActionEvents|InputActionLane_1
  (params (Key :type Key%20Structure :default "AnyKey"))
  (:Pressed
    (CallFunction|ActivateLane 0 true))
  (:Released
    (CallFunction|ActivateLane 0 false)))

(event Input|ActionEvents|InputActionLane_2
  (params (Key :type Key%20Structure :default "AnyKey"))
  (:Pressed
    (CallFunction|ActivateLane 1 true))
  (:Released
    (CallFunction|ActivateLane 1 false)))

(event Input|ActionEvents|InputActionLane_3
  (params (Key :type Key%20Structure :default "AnyKey"))
  (:Pressed
    (CallFunction|ActivateLane 2 true))
  (:Released
    (CallFunction|ActivateLane 2 false)))

(event Input|ActionEvents|InputActionLane_4
  (params (Key :type Key%20Structure :default "AnyKey"))
  (:Pressed
    (CallFunction|ActivateLane 3 true))
  (:Released
    (CallFunction|ActivateLane 3 false)))

(event Input|KeyboardEvents|SpaceBar
  (params (Key :type Key%20Structure :default "AnyKey"))
  (:Pressed
    (bind _outactors (Actor|GetAllActorsOfClass "/Game/Blueprints/BeatPuppets/BeatPuppeteer.BeatPuppeteer_C"))
    (for _array_element _outactors
      (Default|Begin _array_element))))

(event Input|KeyboardEvents|Escape
  (params (Key :type Key%20Structure :default "AnyKey"))
  (:Pressed
    (Game|QuitGame 0 "Quit")))

(fn ConstructionScript)

(fn ActivateLane
  (params (LaneIndex :type Integer) (IsPressing :type Boolean))
  (bind _outactors (Actor|GetAllActorsOfClass "/Game/Blueprints/Main/Highway.Highway_C"))
  (for _array_element _outactors
    (Default|ReceiveLanePress _array_element LaneIndex IsPressing)))