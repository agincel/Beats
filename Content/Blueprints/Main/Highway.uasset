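; Highway is the note track of a four-lane rhythm game, spawning notes from a song hardcoded as a string of 0s and 1s.
; Each Beat event reads the next four characters and spawns a tempo-timed Note in every lane marked 1.
; Overlap regions toggle whether notes can be hit or destroy them.
; Lane presses swap lane materials and destroy hittable notes in that lane, found by searching all Note actors.
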(event OnComponentBeginOverlap(NoteDestroyRegion)
  (params (OtherActor :type Actor%20Object%20Reference) (OtherComp :type Primitive%20Component%20Object%20Reference) (OtherBodyIndex :type Integer) (bFromSweep :type Boolean) (SweepResult :type Hit%20Result%20Structure%20%28by%20ref%29))
  (bind _asnote (Utilities|Casting|CastToNote OtherActor))
  (Actor|DestroyActor _asnote))

(event OnComponentBeginOverlap(NoteHitRegion)
  (params (OtherActor :type Actor%20Object%20Reference) (OtherComp :type Primitive%20Component%20Object%20Reference) (OtherBodyIndex :type Integer) (bFromSweep :type Boolean) (SweepResult :type Hit%20Result%20Structure%20%28by%20ref%29))
  (bind _asnote (Utilities|Casting|CastToNote OtherActor))
  (Variables|/Game/Blueprints/Main/Note.Note_C|SetcanGetHit _asnote true))

(event OnComponentEndOverlap(NoteHitRegion)
  (params (OtherActor :type Actor%20Object%20Reference) (OtherComp :type Primitive%20Component%20Object%20Reference) (OtherBodyIndex :type Integer))
  (bind _asnote (Utilities|Casting|CastToNote OtherActor))
  (Variables|/Game/Blueprints/Main/Note.Note_C|SetcanGetHit _asnote false))

(event EventBeat
  (params (beatDivision :type Integer) (Tempo :type Float%20%28single-precision%29))
  (CallFunction|GetBeat beatDivision Tempo))

(event EventBeginPlay
  (Variables|Default|Setsong (Utilities|String|MakeLiteralString "000000000000000000000000000000001000000000000000000000000000000000000000010000000010000010000000010100000000000000000000101000000000000000000000110000000000000000000000000000000000000000000000000000000000100000000000000000000100000000000000101000000101000000000000000000000000000000000000100000000000000000000000000000000000000001000000001000001000000001010000000000000000000010100000000000000000000011000000000000000000000000000000000000000000000000000000000000001000000000000000011000000000000000110000011000000000000011000000011000000000000000000000000000000000000000000000000000000000000010000000000000000110000000110000011000001100000000000000010000001000000000100000100000000000000000000000000000000000000000000000000000000000000010000000000000000000000000000000000000000100000000100000100000000101000000000000000000001010000000000000000000001100000000000000000000000000000000000000000000000000000000000000100000000000000001000000000000001010000001010000000000000000000000000000000000001000000000000000000000000000000000000000010000000010000010000000010100000000000000000000101000000000000000000000110000000000000000000000000000000000000000000000000000000000000010000000000000000110000000000000001100000110000000000000110000000110000000000000000000000000000000000000000000000000000000000000100000000000000001100000001100000110000011000000000000000100000010000000001000001000")))

(fn ConstructionScript
  (bind _lanes (Variables|Default|GetLanes))
  (bind _notespawners (Variables|Default|GetnoteSpawners))
  (bind _noteends (Variables|Default|GetnoteEnds))
  (Utilities|Array|Clear (Variables|Default|GetnoteSpawners))
  (Utilities|Array|Clear (Variables|Default|GetnoteEnds))
  (Utilities|Array|Clear (Variables|Default|GetLanes))
  (Utilities|FlowControl|Sequence
    (:then_0
      (Utilities|Array|Add _notespawners (Variables|Default|GetnoteSpawn1))
      (Utilities|Array|Add _notespawners (Variables|Default|GetnoteSpawn2))
      (Utilities|Array|Add _notespawners (Variables|Default|GetnoteSpawn3))
      (Utilities|Array|Add _notespawners (Variables|Default|GetnoteSpawn4)))
    (:then_1
      (Utilities|Array|Add _noteends (Variables|Default|GetnoteEnd1))
      (Utilities|Array|Add _noteends (Variables|Default|GetnoteEnd2))
      (Utilities|Array|Add _noteends (Variables|Default|GetnoteEnd3))
      (Utilities|Array|Add _noteends (Variables|Default|GetnoteEnd4)))
    (:then_2
      (Utilities|Array|Add _lanes (Variables|Default|GetLane1))
      (Utilities|Array|Add _lanes (Variables|Default|GetLane2))
      (Utilities|Array|Add _lanes (Variables|Default|GetLane3))
      (Utilities|Array|Add _lanes (Variables|Default|GetLane4)))))

(fn GetBeat
  (params (beatDivision :type Integer) (Tempo :type Float%20%28single-precision%29))
  (LocalVariables|SetcurrentBeat (Utilities|String|GetSubstring (Variables|Default|Getsong) (Variables|Default|GetbeatIndex) 4))
  (for _index (range 0 3)
    (if (Utilities|Enum|Equal(Enum) (Utilities|String|GetSubstring (LocalVariables|GetcurrentBeat) _index) "1")
      (CallFunction|SpawnNote _index Tempo)))
  (Variables|Default|SetbeatIndex (+ (Variables|Default|GetbeatIndex) 4)))

(fn SpawnNote
  (params (lane :type Integer) (Tempo :type Float%20%28single-precision%29))
  (bind _notespawners (Variables|Default|GetnoteSpawners))
  (bind _item (Utilities|Array|Get(acopy) _notespawners lane))
  (bind _returnvalue (Game|SpawnActorfromClass "/Game/Blueprints/Main/Note.Note_C" (Transformation|GetWorldTransform _item) "Undefined" 0 0))
  (Variables|/Game/Blueprints/Main/Note.Note_C|SetstartingTarget _returnvalue _item)
  (Variables|/Game/Blueprints/Main/Note.Note_C|SetendingTarget _returnvalue (Utilities|Array|Get(acopy) (Variables|Default|GetnoteEnds) lane))
  (Variables|/Game/Blueprints/Main/Note.Note_C|SetlerpTime _returnvalue (/ 6e+01 (* Tempo 0.5)))
  (Variables|/Game/Blueprints/Main/Note.Note_C|SetlaneID _returnvalue lane))

(fn ReceiveLanePress
  (params (LaneIndex :type Integer) (IsPressing :type Boolean))
  (if IsPressing
    (Rendering|Material|SetMaterial (Utilities|Array|Get(acopy) (Variables|Default|GetLanes) LaneIndex) 0 (Variables|Default|GetlaneActiveMat))
    (bind _outactors (Actor|GetAllActorsOfClass "/Game/Blueprints/Main/Note.Note_C"))
    (for _array_element _outactors
      (if (and (== (Variables|/Game/Blueprints/Main/Note.Note_C|GetlaneID _array_element) LaneIndex) (Variables|/Game/Blueprints/Main/Note.Note_C|GetcanGetHit _array_element))
        (Actor|DestroyActor _array_element)))
    (else
      (Rendering|Material|SetMaterial (Utilities|Array|Get(acopy) (Variables|Default|GetLanes) LaneIndex) 0 (Variables|Default|GetlaneInactiveMat)))))