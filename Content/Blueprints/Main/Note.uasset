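; Note is an actor that travels in a straight line from a starting target to an ending target over a set duration.
; Each Tick calls Move, which accumulates delta time and sets the actor's location by linearly interpolating between the two targets' current world locations, with sweep enabled.
; The interpolation alpha is elapsed time over LerpTime, with no clamp or arrival handling in the graph.
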(event EventBeginPlay)

(event EventActorBeginOverlap
  (params (OtherActor :type Actor%20Object%20Reference)))

(event EventTick
  (params (DeltaSeconds :type Float%20%28single-precision%29))
  (CallFunction|Move DeltaSeconds))

(fn ConstructionScript)

(fn Move
  (params (deltaTime :type Float%20%28single-precision%29))
  (Variables|Default|SetlerpCurrent (+ (Variables|Default|GetlerpCurrent) deltaTime))
  (Transformation|SetActorLocation (Math|Vector|Lerp(Vector) (Transformation|GetWorldLocation (Variables|Default|GetstartingTarget)) (Transformation|GetWorldLocation (Variables|Default|GetendingTarget)) (/ (Variables|Default|GetlerpCurrent) (Variables|Default|GetlerpTime))) true false))