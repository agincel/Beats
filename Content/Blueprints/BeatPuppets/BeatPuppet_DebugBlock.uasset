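; BeatPuppet_DebugBlock is a debug beat puppet that gives visible and audible feedback on a chosen beat division.
; Its Beat event compares the incoming division to BeatToMoveOn.
; On a match, it randomizes the cube's world rotation and per-axis scale, then plays a 2D beep.
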(event EventBeat
  (params (beatDivision :type Integer) (Tempo :type Float%20%28single-precision%29))
  (bind _cube (Variables|Default|GetCube))
  (if (== beatDivision (Variables|Default|GetbeatToMoveOn))
    (Transformation|SetWorldRotation _cube (Math|Random|RandomRotator true) false false)
    (Transformation|SetWorldScale3D _cube (Math|Vector|MakeVector (Math|Random|RandomFloatinRange 1.0 5.0) (Math|Random|RandomFloatinRange 1.0 5.0) (Math|Random|RandomFloatinRange 1.0 5.0)))
    (Audio|PlaySound2D "/Game/Audio/beep.beep")))

(fn ConstructionScript)