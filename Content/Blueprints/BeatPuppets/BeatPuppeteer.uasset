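; BeatPuppeteer is an actor that plays a music cue and broadcasts its beat to puppet actors.
; Begin activates the audio, then each tick Check Beat compares playback time, adjusted by an offset, against a quarter-beat interval derived from Tempo.
; It fires once immediately when playback starts and cycles a division counter from 0 to 3.
; TriggerBeat sends the division and tempo to every actor implementing BeatPuppet_Interface.
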(event Custom|Begin
  (Components|Activation|Activate (Variables|Default|GetAC) true)
  (Variables|Default|SetBeatTracker 0.0)
  (Variables|Default|SethasUsedFirstBeat false))

(event EventBeginPlay
  (Variables|Default|SetAC (Variables|Default|GetAudio))
  (Audio|Components|Audio|SetSound (Variables|Default|GetAC) (Variables|Default|GetAudioCue)))

(event EventTick
  (params (DeltaSeconds :type Float%20%28single-precision%29))
  (bind _beatdivision (Utilities|CheckBeat)
    (:Did%20Get%20Beat
      (CallFunction|TriggerBeat _beatdivision))))

(fn ConstructionScript)

(fn TriggerBeat
  (params (beatDivision :type Integer))
  (bind _outactors (Actor|GetAllActorswithInterface "/Game/Blueprints/BeatPuppets/BeatPuppet_Interface.BeatPuppet_Interface_C"))
  (for _array_element _outactors
    (Class|BeatPuppetInterface|ReceiveBeat(Message) _array_element beatDivision (Variables|Default|GetTempo))))